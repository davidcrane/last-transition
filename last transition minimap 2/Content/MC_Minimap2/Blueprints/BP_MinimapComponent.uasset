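; BP_MinimapComponent is a component that puts the minimap on screen when play begins.
; It creates a BP_Minimap widget for player controller 0, stores the reference and adds it to the viewport.
; It then copies its own zoom-when-hovered and zoom scale settings onto the widget, so minimap zoom is configured from the component.
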(event `self.ReceiveBeginPlay`
  (`|ExecutionSequence`
    (:`then_0`
      ;[1 1 1] Create minimap widget
      (bind _returnvalue (`|CreateWidget` "/Game/MC_Minimap2/Blueprints/BP_Minimap.BP_Minimap_C" (`GameplayStatics.GetPlayerController` 0)))
      (bind _output_get (set `self.MinimapWidget` _returnvalue))
      (`UserWidget.AddToViewport` _output_get 0)
      ;[1 1 1] Set zoom when hovered
      (set `/Game/MC_Minimap2/Blueprints/BP_Minimap.ZoomWhenHovered` (`self.ZoomWhenHovered`) (`self.MinimapWidget`))
      ;[1 1 1] Set zoom scale
      (set `/Game/MC_Minimap2/Blueprints/BP_Minimap.ZoomScale` (`self.ZomScale`) (`self.MinimapWidget`)))))